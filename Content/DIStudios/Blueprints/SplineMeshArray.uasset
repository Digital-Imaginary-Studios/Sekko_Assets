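; SplineMeshArray is a construction-script actor that builds a chain of deformed meshes along a spline.
; Each segment between spline points gets a spline mesh with a random, unseeded pick from the Mesh array and a configurable forward axis.
; Segment ends follow point locations and tangents, offset by Spacing along the spline component's forward vector rather than each segment's direction.
; Meshes use query-only collision.
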(event EventBeginPlay)

(event Collision|EventActorBeginOverlap
  (params (OtherActor :type Actor%20Object%20Reference)))

(event EventTick
  (params (DeltaSeconds :type Float%20%28single-precision%29)))

(fn ConstructionScript
  (bind _mesh (Variables|Default|GetMesh))
  (bind _spline (Variables|Components|GetSpline))
  (bind _spacing (Variables|Default|GetSpacing))
  (bind _returnvalue (Math|Vector|GetForwardVector _spline))
  (bind _returnvalue_2 (* _returnvalue _spacing))
  (for _index (range 0 (- (Spline|GetNumberOfSplinePoints _spline) 2))
    (bind _returnvalue_3 (AddComponent|AddSplineMeshComponent false))
    (Components|StaticMesh|SetStaticMesh _returnvalue_3 (Utilities|Array|Get(acopy) _mesh (Math|Random|RandomIntegerinRange 0 (- (Utilities|Array|Length _mesh) 1))))
    (SplineMesh|SetForwardAxis _returnvalue_3 (Variables|Default|GetForward%20Axis) true)
    (Transformation|AttachComponentToComponent _returnvalue_3 _spline "None" "KeepRelative" "KeepRelative" "KeepRelative" true)
    (SplineMesh|SetStartandEnd _returnvalue_3 (- (Spline|GetLocationatSplinePoint _spline _index "Local") _returnvalue_2) (Spline|GetTangentatSplinePoint _spline _index "Local") (+ (Spline|GetLocationatSplinePoint _spline (+ _index 1) "Local") _returnvalue_2) (Spline|GetTangentatSplinePoint _spline (+ _index 1) "Local") true :!class /Script/Engine.SplineMeshComponent)
    (Collision|SetCollisionEnabled _returnvalue_3 "QueryOnly")))